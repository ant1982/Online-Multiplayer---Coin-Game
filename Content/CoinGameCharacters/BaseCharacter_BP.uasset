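; Base character Blueprint for the coin game that tints the character's body to show its team.
; Shortly after BeginPlay, the server reads the team number and sets the Colour RepNotify variable to red for team 1 or blue for team 2.
; OnRep_Colour creates a dynamic instance of the mannequin body material on the mesh and applies the colour to its BodyColor parameter.
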(event `self.ReceiveBeginPlay`
  (`KismetSystemLibrary.Delay` 0.2)
  (`/Engine/EditorBlueprintResources/ActorMacros.Switch Has Authority`
    (:`Authority`
      (bind _returnvalue (`self.GetTeamNumber` self))
      (switch `int` _returnvalue
        (:`1`
          (set `self.Colour` (make `LinearColor` 0.9 0.0 0.0 1.0)))
        (:`2`
          (set `self.Colour` (make `LinearColor` 0.0 0.0 0.9 1.0)))))))

(fn `OnRep_Colour`
  (bind _returnvalue (`PrimitiveComponent.CreateDynamicMaterialInstance` (`self.Mesh`) 0 "/Game/Mannequin/Character/Materials/M_UE4Man_Body.M_UE4Man_Body" "None"))
  (`MaterialInstanceDynamic.SetVectorParameterValue` _returnvalue "BodyColor" (`self.Colour`)))

(fn `UserConstructionScript`)